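; Player-flown airplane pawn that constantly moves forward and is steered with Enhanced Input.
; Tick feeds forward movement input and spins the left and right propellers through the custom event RotatePropller; an identical RotatePropeller function exists but is not called here.
; IA_PitchRoll applies frame-rate-scaled local pitch and roll rotation to the actor.
; IA_Fire only prints a debug string, with no firing logic yet.
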(event Custom|RotatePropller
  (params (where :type Static%20Mesh%20Component%20Object%20Reference))
  ;[1 1 1] 커스텀이벤트는 반환값이 없는 함수 네트워크에 필수 함수는 네트워크할때 호출 불가
  (Transformation|AddRelativeRotation where (Math|Rotator|MakeRotator (* (Utilities|Time|GetWorldDeltaSeconds) (Variables|Default|GetPropellerSpeed)) 0.0 0.0) false false))

(event Input|EnhancedActionEvents|EnhancedInputActionIA_Pitch
  (params (ActionValue :type Float%20%28double-precision%29) (ElapsedSeconds :type Float%20%28double-precision%29) (TriggeredSeconds :type Float%20%28double-precision%29) (InputAction :type Input%20Action%20Object%20Reference :default "/Game/Airplane/Blueprints/Input/IA_Pitch.IA_Pitch"))
  ;[1 1 1] Pitch축 회전
)

(event Input|EnhancedActionEvents|EnhancedInputActionIA_Roll
  (params (ActionValue :type Float%20%28double-precision%29) (ElapsedSeconds :type Float%20%28double-precision%29) (TriggeredSeconds :type Float%20%28double-precision%29) (InputAction :type Input%20Action%20Object%20Reference :default "/Game/Airplane/Blueprints/Input/IA_Roll.IA_Roll"))
  ;[1 1 1] Roll축회전
)

(event Input|EnhancedActionEvents|EnhancedInputActionIA_PitchRoll
  (params (ActionValue :type Vector%202D%20Structure) (ElapsedSeconds :type Float%20%28double-precision%29) (TriggeredSeconds :type Float%20%28double-precision%29) (InputAction :type Input%20Action%20Object%20Reference :default "/Game/Airplane/Blueprints/Input/IA_PitchRoll.IA_PitchRoll"))
  (:Triggered
    (Transformation|AddActorLocalRotation (* (Math|Rotator|MakeRotator (.x ActionValue) (.y ActionValue) 0.0) (* (Utilities|Time|GetWorldDeltaSeconds) (Variables|Default|GetRotateSpeed))) false false)))

(event Input|EnhancedActionEvents|EnhancedInputActionIA_Fire
  (params (ActionValue :type Boolean) (ElapsedSeconds :type Float%20%28double-precision%29) (TriggeredSeconds :type Float%20%28double-precision%29) (InputAction :type Input%20Action%20Object%20Reference :default "/Game/Airplane/Blueprints/Input/IA_Fire.IA_Fire"))
  (:Triggered
    (Development|PrintString "Fire")))

(event EventTick
  (params (DeltaSeconds :type Float%20%28single-precision%29))
  (Utilities|FlowControl|Sequence
    (:then_0
      ;[1 1 1] 앞으로 전진
      (Pawn|Input|AddMovementInput (Transformation|GetActorForwardVector) 1.0 false))
    (:then_1
      ;[1 1 1] 왼쪽프로펠러 회전
      (CallFunction|RotatePropller (Variables|Default|GetLeft)))
    (:then_2
      ;[1 1 1] 오른쪽프로펠러 회전
      (CallFunction|RotatePropller (Variables|Default|GetRight)))))

(fn ConstructionScript)

(fn RotatePropeller
  (params (where :type Scene%20Component%20Object%20Reference))
  (Transformation|AddRelativeRotation where (Math|Rotator|MakeRotator (* (Utilities|Time|GetWorldDeltaSeconds) (Variables|Default|GetPropellerSpeed)) 0.0 0.0) false false))